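; BP_CameraPlayer is a player-controlled camera pawn with floating movement and stepped zoom.
; Enhanced Input actions move it along its forward and right vectors, while the acceleration action doubles FloatingPawnMovement's max speed when started and halves it on release or cancel.
; Zoom input accumulates into a clamped step count, which offsets the SpringArm's socket from the position cached at BeginPlay rather than changing arm length.
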(event Input|EnhancedActionEvents|EnhancedInputActionIA_MoveForward
  (params (ActionValue :type Float%20%28double-precision%29) (ElapsedSeconds :type Float%20%28double-precision%29) (TriggeredSeconds :type Float%20%28double-precision%29) (InputAction :type Input%20Action%20Object%20Reference :default "/Game/Blueprint/Player/Inputs/IA_MoveForward.IA_MoveForward"))
  (Pawn|Input|AddMovementInput (Transformation|GetActorForwardVector) ActionValue false))

(event Input|EnhancedActionEvents|EnhancedInputActionIA_MoveSide
  (params (ActionValue :type Float%20%28double-precision%29) (ElapsedSeconds :type Float%20%28double-precision%29) (TriggeredSeconds :type Float%20%28double-precision%29) (InputAction :type Input%20Action%20Object%20Reference :default "/Game/Blueprint/Player/Inputs/IA_MoveSide.IA_MoveSide"))
  (Pawn|Input|AddMovementInput (Transformation|GetActorRightVector) ActionValue false))

(event Input|EnhancedActionEvents|EnhancedInputActionIA_Zoom
  (params (ActionValue :type Float%20%28double-precision%29) (ElapsedSeconds :type Float%20%28double-precision%29) (TriggeredSeconds :type Float%20%28double-precision%29) (InputAction :type Input%20Action%20Object%20Reference :default "/Game/Blueprint/Player/Inputs/IA_Zoom.IA_Zoom"))
  (:Triggered
    (bind _output_get (Variables|Default|SetZoomSteps (Math|Integer|Clamp(Integer) (+ (Math|Float|Floor ActionValue) (Variables|Default|GetZoomSteps)) 0 20)))
    (Variables|/Script/Engine.SpringArmComponent|SetSocketOffset (Variables|Default|GetSpringArm) (+ (* _output_get (Variables|Default|GetZoomOffsetPerStep)) (Variables|Default|GetStartArmPosition)))))

(event Input|EnhancedActionEvents|EnhancedInputActionIA_Aceleration
  (params (ActionValue :type Boolean) (ElapsedSeconds :type Float%20%28double-precision%29) (TriggeredSeconds :type Float%20%28double-precision%29) (InputAction :type Input%20Action%20Object%20Reference :default "/Game/Blueprint/Player/Inputs/IA_Aceleration.IA_Aceleration"))
  (bind _floatingpawnmovement (Variables|Default|GetFloatingPawnMovement))
  (bind _floatingpawnmovement_2 (Variables|Default|GetFloatingPawnMovement))
  (:Started
    (Variables|/Script/Engine.FloatingPawnMovement|SetMaxSpeed _floatingpawnmovement (* 2.0 (Class|MovementComponent|GetMaxSpeed _floatingpawnmovement))))
  (:Canceled
    (Variables|/Script/Engine.FloatingPawnMovement|SetMaxSpeed _floatingpawnmovement_2 (* 0.5 (Class|MovementComponent|GetMaxSpeed _floatingpawnmovement_2)) :!label _label))
  (:Completed
    (goto _label)))

(event EventBeginPlay
  (Variables|Default|SetStartArmPosition (Variables|/Script/Engine.SpringArmComponent|GetSocketOffset (Variables|Default|GetSpringArm))))

(event Collision|EventActorBeginOverlap
  (params (OtherActor :type Actor%20Object%20Reference)))

(event EventTick
  (params (DeltaSeconds :type Float%20%28single-precision%29)))

(fn ConstructionScript)