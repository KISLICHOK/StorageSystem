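; BP_StoragePreGameBuilder is an actor that places a grid of storage actors when play begins and registers them as prepared builds.
; CreateStorages spawns StorageClass instances from the builder's location, spaced by X and Y cell counts and sizes with no rotation, and collects valid spawns in Storages.
; BeginPlay then passes each valid storage to STWorldBuildSubsystem through AddPreparedBuild.
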(event EventBeginPlay
  (Utilities|FlowControl|Sequence
    (:then_0
      (CallFunction|CreateStorages))
    (:then_1
      ;[1 1 1] Add Prepeared build in storage
      (for _array_element (Variables|Default|GetStorages)
        (Utilities|IsValid _array_element
          (:Is%20Valid
            (Class|STWorldBuildSubsystem|AddPreparedBuild (Subsystems|GetSTWorldBuildSubsystem) _array_element)))))))

(fn ConstructionScript)

(fn CreateStorages
  (for _index (range 0 (Variables|Default|GetXCount))
    (for _index_2 (range 0 (Variables|Default|GetYCount))
      (bind _returnvalue (Game|SpawnActorfromClass (Variables|Default|GetStorageClass) (Math|Transform|MakeTransform (+ (Transformation|GetActorLocation) (Math|Vector|MakeVector (* _index (Variables|Default|GetXCellSize)) (* _index_2 (Variables|Default|GetYCellSize)) 0.0))) "Undefined" "MultiplyWithRoot" 0 0))
      (Utilities|IsValid _returnvalue
        (:Is%20Valid
          (Utilities|Array|Add (Variables|Default|GetStorages) _returnvalue))))))