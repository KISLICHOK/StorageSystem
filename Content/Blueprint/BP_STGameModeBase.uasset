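; Game mode base that starts the ST game session and wires up building selection when play begins.
; BeginPlay starts the world loader and world build subsystems, then spawns a BP_BuildSelectController.
; That spawned controller is handed to the first player's BP_STPlayerController and to its BP_STGameHUD, so both share one instance.
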(event EventBeginPlay
  (Utilities|FlowControl|Sequence
    (:then_0
      (Class|STWorldLoadersSubsystem|StartGame (Subsystems|GetBPSTWorldLoaderSubsystem))
      (Class|STWorldBuildSubsystem|StartGame (Subsystems|GetBPSTWorldBuildSubsystem))
      (bind _returnvalue (Game|SpawnActorfromClass "/Game/Blueprint/Controllers/BP_BuildSelectController.BP_BuildSelectController_C" (Math|Transform|MakeTransform "0, 0, 0" "0, 0, 0" "1.000000,1.000000,1.000000") "Undefined" "MultiplyWithRoot" 0 0))
      (Variables|Default|SetSpawnController _returnvalue))
    (:then_1
      (bind _asbp_stplayer_controller (Utilities|Casting|CastToBP_STPlayerController (Game|GetPlayerController 0)))
      (bind _output_get (Variables|Default|SetSTPlayerController _asbp_stplayer_controller))
      (Variables|/Game/Blueprint/Player/BP_STPlayerController.BP_STPlayerController_C|SetSpawnController _output_get (Variables|Default|GetSpawnController)))
    (:then_2
      (bind _asbp_stgame_hud (Utilities|Casting|CastToBP_STGameHUD (HUD|GetHUD (Variables|Default|GetSTPlayerController))))
      (bind _output_get_2 (Variables|Default|SetBPSTGame%20HUD _asbp_stgame_hud))
      (Variables|/Game/UI/HUDs/BP_STGameHUD.BP_STGameHUD_C|SetSpawnController _output_get_2 (Variables|Default|GetSpawnController)))))

(event EventTick
  (params (DeltaSeconds :type Float%20%28single-precision%29)))

(fn ConstructionScript)