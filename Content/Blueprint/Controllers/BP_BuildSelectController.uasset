(fn ConstructionScript)

(fn SetNewUIInfo
  (params (StorageInfo :type Storage%20UI%20Info%20Structure))
  (Utilities|IsValid (Variables|Default|GetSelectedStorage)
    (:Is%20Not%20Valid
      (bind _output_get (Variables|Default|SetStorageUIInfo StorageInfo))
      (Default|CallSetNewUIInfoDispatcher _output_get))))

(fn SelectStorage
  (params (Storage :type BP%20ST%20Storage%20Build%20Object%20Reference))
  (CallFunction|UnSelectStorage)
  (bind _output_get (Variables|Default|SetSelectedStorage Storage))
  (EventDispatchers|BindEventtoOnCurrentResourcesChangedbyPlayer _output_get (EventDispatchers|CreateEvent :!event StorageInfoChanged))
  (Default|CallSelectStorageEventDispatcher _output_get)
  (Default|CallSetNewUIInfoDispatcher (Class|STStorageBuild|GetUIInfo _output_get))
  (EventDispatchers|BindEventtoOnChangeUIInfo (Variables|Default|GetSelectedStorage) (EventDispatchers|CreateEvent :!event SetNewUIInfo)))

(fn StorageInfoChanged
  (params (StorageInfo :type Storage%20Info%20Structure))
  (Default|CallSetNewUIInfoDispatcher (Utilities|Struct|MakeStorageUIInfo (.storageid StorageInfo) (.maxresourcecount StorageInfo) (.resourcetype StorageInfo) (.loadcount StorageInfo))))

(fn UnSelectStorage
  (Utilities|IsValid (Variables|Default|GetSelectedStorage)
    (:Is%20Valid
      (EventDispatchers|UnbindEventfromOnCurrentResourcesChangedbyPlayer (Variables|Default|GetSelectedStorage) (EventDispatchers|CreateEvent self :!event StorageInfoChanged))
      (Variables|Default|SetSelectedStorage 0)
      (Default|CallUnSelectStorageEventDispatcher))))

(fn OnPlayerAddResource
  (bind _selectedstorage (Variables|Default|GetSelectedStorage))
  (Utilities|IsValid _selectedstorage
    (:Is%20Valid
      (Class|STStorageBuild|AddResource _selectedstorage 1))))

(fn OnPlayerRemoveResource
  (bind _selectedstorage (Variables|Default|GetSelectedStorage))
  (Utilities|IsValid _selectedstorage
    (:Is%20Valid
      (Class|STStorageBuild|AddResource _selectedstorage -1))))

(fn OnCreateLoader
  (Class|STWorldLoadersSubsystem|CreateDefaultLoader (Subsystems|GetBPSTWorldLoaderSubsystem) (Math|Transform|MakeTransform "-200.000000,-200.000000,0.000000" "0, 0, 0" "1.000000,1.000000,1.000000")))

(fn OnCreateStorage
  (Default|CallCreateStorageEventDispatcher))

(fn StartStressUpdate
  (Class|STWorldBuildSubsystem|StressUpdateStorages (Subsystems|GetBPSTWorldBuildSubsystem)))

(fn OnStressTestBegin
  (CallFunction|StartStressUpdate))

(fn NewFunction)

(fn OnResourceTypeChanged
  (params (RecourceType :type EResourceType%20Enum :default "ResourceType1"))
  (bind _output_get (Variables|StorageSettings|SetStorageResourceType RecourceType))
  (Development|PrintString (Utilities|String|EnumtoString _output_get)))

(fn OnStorageCapacityChanged
  (params (NewParam :type Integer))
  (Variables|StorageSettings|SetStorageCapacity NewParam))

(fn CreateStorage
  (params (Location :type Vector))
  (Class|STWorldBuildSubsystem|CreateNewStorage (Subsystems|GetBPSTWorldBuildSubsystem) "/Game/Blueprint/Builds/BP_STStorageBuild.BP_STStorageBuild_C" (Math|Transform|MakeTransform Location "0, 0, 0" "1.000000,1.000000,1.000000") (Variables|StorageSettings|GetStorageResourceType) (+ (Variables|StorageSettings|GetStorageCapacity) 1)))