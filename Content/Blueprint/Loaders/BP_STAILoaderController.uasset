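; AI controller that drives STLoader pawns to the target locations of their load-carrying orders.
; On possess it binds to the loader's start-take-load and start-bring-load events.
; Both handlers run AIMoveTo toward the loader's current target location and call ReachedDestination on the loader when the move succeeds.
; Failed moves have no handling.
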(event Custom|OnStartBringLoad_Event
  (params (Loader :type ST%20Loader%20Object%20Reference) (Order :type Load%20Order%20Structure))
  (bind _returnvalue (Class|STLoader|GetTargetLocation Loader))
  (AI|AIMoveTo 0 _returnvalue 0 3e+01 true
    (:OnSuccess
      (Class|STLoader|ReachedDestination Loader))))

(event Custom|OnStartTakeLoad_Event
  (params (Loader :type ST%20Loader%20Object%20Reference) (Order :type Load%20Order%20Structure))
  (bind _returnvalue (Class|STLoader|GetTargetLocation Loader))
  (AI|AIMoveTo 0 _returnvalue 0 3e+01 true
    (:OnSuccess
      (Class|STLoader|ReachedDestination Loader))))

(event EventPossess
  (params (PossessedPawn :type Pawn%20Object%20Reference))
  (bind _asstloader (Utilities|Casting|CastToSTLoader PossessedPawn))
  (EventDispatchers|BindEventtoOnStartTakeLoad _asstloader (delegate Custom|OnStartTakeLoad_Event))
  (EventDispatchers|BindEventtoOnStartBringLoad _asstloader (delegate Custom|OnStartBringLoad_Event)))

(fn ConstructionScript)